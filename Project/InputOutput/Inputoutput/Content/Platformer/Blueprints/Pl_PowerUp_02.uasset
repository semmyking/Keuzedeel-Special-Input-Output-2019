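; Super jump pickup for a platformer that temporarily raises the player character's jump velocity.
; Any actor overlap removes the mesh and box, boosts player 0, then after a delay sets a hardcoded normal jump value, with debug prints for both states.
; The actor itself is never destroyed and spins by a fixed step every Tick, so rotation speed depends on frame rate.
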(event `self.ReceiveActorBeginOverlap`
  (params (OtherActor :type "Actor Object Reference"))
  (bind _charactermovement (`Character.CharacterMovement` (`GameplayStatics.GetPlayerCharacter` 0)))
  (`ActorComponent.K2_DestroyComponent` (`self.StaticMesh`))
  (`ActorComponent.K2_DestroyComponent` (`self.Box`))
  (`KismetSystemLibrary.PrintString` "SuperJump")
  (set `CharacterMovementComponent.JumpZVelocity` 1200.0 _charactermovement)
  (`KismetSystemLibrary.Delay` 5.0)
  (set `CharacterMovementComponent.JumpZVelocity` 600.0 _charactermovement)
  (`KismetSystemLibrary.PrintString` "NormalJump"))

(event `self.ReceiveTick`
  (params (DeltaSeconds :type "Float (single-precision)"))
  (`self.K2_AddActorLocalRotation` (struct :`Yaw` 5.0)))

(fn `UserConstructionScript`)