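; Platformer super-jump power-up pickup that temporarily boosts the player character's jump.
; On any actor overlap it destroys its mesh and sphere, raises player 0's JumpZVelocity, then restores a hardcoded normal value after a short delay.
; The actor itself is never destroyed, and debug strings print on each change.
; A separate event taking DeltaSeconds spins the actor by a fixed, frame-rate-dependent step.
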(event `self.ReceiveActorBeginOverlap`
  (params (OtherActor :type "Actor Object Reference"))
  (bind _charactermovement (`Character.CharacterMovement` (`GameplayStatics.GetPlayerCharacter` 0)))
  (`ActorComponent.K2_DestroyComponent` (`self.StaticMesh`))
  (`ActorComponent.K2_DestroyComponent` (`self.Sphere`))
  (`KismetSystemLibrary.PrintString` "SuperJump")
  (set `CharacterMovementComponent.JumpZVelocity` 2000.0 _charactermovement)
  (`KismetSystemLibrary.Delay` 2.0)
  (set `CharacterMovementComponent.JumpZVelocity` 600.0 _charactermovement)
  (`KismetSystemLibrary.PrintString` "NormalJump"))

(event `CustomEvent`
  (params (DeltaSeconds :type "Float (double-precision)"))
  (`self.K2_AddActorLocalRotation` (struct :`Yaw` 5.0)))

(fn `UserConstructionScript`)